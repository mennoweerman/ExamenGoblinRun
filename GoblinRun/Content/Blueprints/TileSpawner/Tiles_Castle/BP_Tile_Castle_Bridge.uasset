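; Castle bridge tile for the tile spawner, which seeds the surrounding tiles when the player starts inside it.
; BeginPlay waits one tick, then tests the detection collision against the player pawn, since begin overlap misses a player spawned inside.
; On overlap it calls SpawnAdjacentTiles, then repeats that call on NewTiles entries for SpawnRadius-driven passes, removing entries mid-loop and finally clearing the array.
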(event EventBeginPlay
  (bind _newtiles (Variables|Default|GetNewTiles))
  ;[1 1 1] Check if the starting tile is overlapping with the player, since begin overlap does not work when the player is spawned inside it.
  (|CallParentFunction)
  (Utilities|FlowControl|DelayUntilNextTick)
  (if (Collision|IsOverlappingActor (Variables|Default|GetCollision_PlayerDetection) (Game|Player|GetPlayerPawn 0) :!class /Script/Engine.PrimitiveComponent)
    (CallFunction|SpawnAdjacentTiles)
    (for _index (range 0 (Variables|Default|GetSpawnRadius))
      (for _array_element _newtiles
        (Default|SpawnAdjacentTiles _array_element)
        (Utilities|Array|RemoveItem _newtiles _array_element)))
    (Utilities|Array|Clear _newtiles)))

(event Collision|EventActorBeginOverlap
  (params (OtherActor :type Actor%20Object%20Reference))
  (|CallParentFunction OtherActor) ; This node is disabled and will not be called.\nDrag off pins to build functionality.
)

(event EventTick
  (params (DeltaSeconds :type Float%20%28single-precision%29))
  (|CallParentFunction DeltaSeconds) ; This node is disabled and will not be called.\nDrag off pins to build functionality.
)

(fn ConstructionScript
  (|CallParentFunction))