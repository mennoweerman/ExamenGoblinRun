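; Procedural world tile that spawns matching neighbours as the player moves and destroys itself beyond a despawn distance.
; Player overlap triggers spawning at four edge spawnpoints, repeated over newly spawned tiles by SpawnRadius.
; Each edge's land, road or water type selects candidate classes from BP_TileManager for the opposite side.
; Where spawnpoints overlap, it intersects their candidate lists and spawns a random match, falling back to BackupTile.
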(event OnComponentBeginOverlap(Collision_PlayerDetection)
  (params (OverlappedComponent :type Primitive%20Component%20Object%20Reference) (OtherActor :type Actor%20Object%20Reference) (OtherComp :type Primitive%20Component%20Object%20Reference) (OtherBodyIndex :type Integer) (bFromSweep :type Boolean) (SweepResult :type Hit%20Result%20Structure%20%28by%20ref%29))
  (bind _newtiles (Variables|Spawning|GetNewTiles))
  ;[1 1 1] When the player starts overlapping a tile, the ones surrounding it are spawned in.
  (if (== OtherActor (Variables|References|GetPlayerRef))
    (CallFunction|SpawnAdjacentTiles)
    (for _index (range 0 (Variables|Spawning|GetSpawnRadius))
      (for _array_element _newtiles
        (CallFunction|SpawnAdjacentTiles _array_element)
        (Utilities|Array|RemoveItem _newtiles _array_element)))
    (Utilities|Array|Clear _newtiles)))

(event EventBeginPlay
  (bind _spawnpoints (Variables|Spawning|GetSpawnpoints))
  ;[1 1 1] On begin play, the player is set and the spawnpoints are added to the array.
  (bind _returnvalue (Actor|GetActorOfClass "/Game/Blueprints/TileSpawner/Blueprints_Other/BP_TileManager.BP_TileManager_C"))
  (Variables|References|SetTileManagerRef _returnvalue)
  (bind _output_get (Variables|References|SetPlayerRef (Game|Player|GetPlayerPawn 0)))
  (Utilities|IsValid _output_get
    (:Is%20Valid
      (Utilities|Array|Add _spawnpoints (Variables|Default|GetSpawn_Top))
      (Utilities|Array|Add _spawnpoints (Variables|Default|GetSpawn_Right))
      (Utilities|Array|Add _spawnpoints (Variables|Default|GetSpawn_Bottom))
      (Utilities|Array|Add _spawnpoints (Variables|Default|GetSpawn_Left)))
    (:Is%20Not%20Valid
      (Development|PrintString "Warning! Player not set in BP_Tile!" true true "(R=1.000000,G=1.000000,B=0.000000,A=1.000000)" 25.0))))

(event EventTick
  (params (DeltaSeconds :type Float%20%28single-precision%29))
  ;[1 1 1] Checks if the player is further from a tile than the despawn distance and destroys the tile. Tick interval increased to 3 seconds.
  (if (>= (Transformation|GetDistanceTo (Variables|References|GetPlayerRef) self) (Variables|Despawning|GetDespawnDistance))
    (Actor|DestroyActor)))

(fn ConstructionScript)

(fn SpawnAdjacentTiles
  (bind _tilesinallarrays (Variables|Spawning|GetTilesInAllArrays))
  ;[1 1 1] Spawns tiles on the spawnpoints that aren't colliding with anything, with the exception of another spawnpoint.
  ;;[0 0 0] Loops through all the spawnpoints of a tile.
  (for (_array_element _array_index) (Variables|Spawning|GetSpawnpoints)
    (LocalVariables|SetSpawnpoint _array_element)
    (LocalVariables|SetSpawnpointIndex _array_index)
    ;;[0 0 0] Check if spawnpoint isn't overlapping with any tile blueprints.
    (if (Utilities|Array|IsEmpty (Collision|GetOverlappingActors (LocalVariables|GetSpawnpoint) "BP_Tile_C" :!class /Script/Engine.PrimitiveComponent))
      ;;[0 0 0] If not, a new tile is spawned.
      (bind _spawnabletiles (CallFunction|GetSpawnableTiles (Variables|Spawning|GetPossibleTileConnections) (LocalVariables|GetSpawnpointIndex)))
      (CallFunction|SpawnRandomTilefromArray _spawnabletiles (LocalVariables|GetSpawnpoint))
      (else
        ;;[0 0 0] If this spawnpoint is already overlapping with something else in the tile blueprint, this makes sure that it is only another spawnpoint, and not another tile, as you wouldn't want to spawn a tile on top of an existing one.
        (Utilities|Array|Clear (Variables|Spawning|GetOverlappingSpawnpoints))
        (bind _array_element_2 (Utilities|Array|ForEachLoopwithBreak (Class|PrimitiveComponent|GetOverlappingComponents (LocalVariables|GetSpawnpoint)) :!label _label)
          (:LoopBody
            (bind _output_get (LocalVariables|SetOverlappedComponent _array_element_2))
            (bind _output_get_2 (Variables|Spawning|SetContainsOnlySpawnpoints? (Components|ComponentHasTag _output_get "SpawnPoint")))
            (if _output_get_2
              (Utilities|Array|Add (Variables|Spawning|GetOverlappingSpawnpoints) (LocalVariables|GetOverlappedComponent))
              (else
                (goto _label Break))))
          (:Completed
            (if (Variables|Spawning|GetContainsOnlySpawnpoints?)
              ;[1 1 1] Sequence of events that make sure a new tile is spawned on a spawnpoint that contains overlapping spawnpoints.
              ;;[0 0 0] For each spawnpoint overlapping with this current spawnpoint, gets the tag index to know wether that one is Top, Right, Bottom or Left.
              (Utilities|Array|Clear (Variables|Spawning|GetCompatibleTileArrays))
              (for _array_element_3 (Variables|Spawning|GetOverlappingSpawnpoints)
                (for (_array_element_4 _array_index_2) (Variables|Spawning|GetPossibleTags)
                  (if (Components|ComponentHasTag _array_element_3 _array_element_4)
                    ;;[0 0 0] Possible tile connection arrays for the overlapping spawnpoints are added to the array of possible tile connection arrays.
                    (bind _asbp_tile (Utilities|Casting|CastToBP_Tile (Components|GetOwner _array_element_3)))
                    (bind _spawnabletiles_2 (CallFunction|GetSpawnableTiles (Variables|BP_Tile_C|GetPossibleTileConnections _asbp_tile) _array_index_2))
                    (Utilities|Array|Add (Variables|Spawning|GetCompatibleTileArrays) (Utilities|Struct|MakeE_SpawnableTileArrays _spawnabletiles_2)))))
              ;;[0 0 0] Gets the possible connections of the current spawnpoint, loops through them and loops through all the possible connections of every overlapping spawnpoint, checks which ones they have in common and adds them to a new array.
              (bind _spawnabletiles_3 (CallFunction|GetSpawnableTiles (Variables|Spawning|GetPossibleTileConnections) (LocalVariables|GetSpawnpointIndex)))
              (for _array_element_5 _spawnabletiles_3
                (bind _array_element_6 (Utilities|Array|ForEachLoopwithBreak (Variables|Spawning|GetCompatibleTileArrays) :!label _label_2)
                  (:LoopBody
                    (bind _output_get_3 (LocalVariables|SetContainsSameTile? (Utilities|Array|ContainsItem (.tilearray _array_element_6) _array_element_5)))
                    (if (not _output_get_3)
                      (goto _label_2 Break)))
                  (:Completed
                    (if (LocalVariables|GetContainsSameTile?)
                      (Utilities|Array|Add (Variables|Spawning|GetTilesInAllArrays) _array_element_5)))))
              ;;[0 0 0] If they have tiles in common, a random one of these is spawned.
              (if (Utilities|Array|IsNotEmpty _tilesinallarrays)
                _
                (else
                  (Utilities|Array|Add _tilesinallarrays (Variables|Spawning|GetBackupTile))))
              (CallFunction|SpawnRandomTilefromArray _tilesinallarrays (LocalVariables|GetSpawnpoint))
              (Utilities|Array|Clear (Variables|Spawning|GetTilesInAllArrays))
              (Utilities|Array|Clear (Variables|Spawning|GetCompatibleTileArrays))))))))
  (return))

(fn SpawnRandomTilefromArray
  (params (ArrayOfTiles :type Array%20of%20BP%20Tile%20Class%20References) (Spawnpoint :type Scene%20Component%20Object%20Reference))
  ;[1 1 1] Spawns a random tile on a spawnpoint from the array.
  (bind _returnvalue (Game|SpawnActorfromClass (Utilities|Array|Get(acopy) ArrayOfTiles (Math|Random|RandomInteger (- (Utilities|Array|Length ArrayOfTiles) 1))) (Math|Transform|MakeTransform (Transformation|GetWorldLocation Spawnpoint) "0, 0, 0" "1.000000,1.000000,1.000000") "AlwaysSpawn" "OverrideRootScale" 0 0))
  (Utilities|Array|Add (Variables|Spawning|GetNewTiles) _returnvalue)
  (return))

(fn GetSpawnableTiles
  (params (PossibleTileConnections :type Map%20of%20E_TileSides%20Enums%20to%20Structs :default "NewEnumerator4") (SpawnpointIndex :type Integer))
  (bind _returnvalue (Utilities|Select :Index SpawnpointIndex :Option%200 2 :Option%201 3 :Option%202 0 :Option%203 1))
  ;[1 1 1] Returns an array of the tile classes that can be attached to a specific spawnpoint.
  (bind _values (Utilities|Map|Values PossibleTileConnections))
  (if (.land (Utilities|Array|Get(acopy) _values SpawnpointIndex))
    (bind _values_2 (Utilities|Map|Values (Variables|/Game/Blueprints/TileSpawner/Blueprints_Other/BP_TileManager.BP_TileManager_C|GetTilesLand (Variables|References|GetTileManagerRef))))
    (return (.possibleadjacenttiles (Utilities|Array|Get(acopy) _values_2 _returnvalue)))
    (elif (.road (Utilities|Array|Get(acopy) _values SpawnpointIndex))
      (bind _values_3 (Utilities|Map|Values (Variables|/Game/Blueprints/TileSpawner/Blueprints_Other/BP_TileManager.BP_TileManager_C|GetTilesRoad (Variables|References|GetTileManagerRef))))
      (return (.possibleadjacenttiles (Utilities|Array|Get(acopy) _values_3 _returnvalue)))
      (else
        (bind _values_4 (Utilities|Map|Values (Variables|/Game/Blueprints/TileSpawner/Blueprints_Other/BP_TileManager.BP_TileManager_C|GetTilesWater (Variables|References|GetTileManagerRef))))
        (return (.possibleadjacenttiles (Utilities|Array|Get(acopy) _values_4 _returnvalue)))))))