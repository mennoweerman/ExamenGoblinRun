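; BP_BasicEnemy is a basic enemy pawn that chases the first player and removes itself after a set lifetime.
; On BeginPlay, one timer sets the capsule's object type to Pawn and makes it block WorldStatic after a short delay.
; A second timer destroys the actor once DespawnTime elapses.
; Every Tick reissues an AIMoveTo toward the player pawn.
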(event Custom|SetCollision
  (bind _capsulecomponent (Variables|Collision|GetCapsuleComponent))
  ;[1 1 1] Reset collision
  (Collision|SetCollisionObjectType _capsulecomponent "ECC_Pawn")
  (Collision|SetCollisionResponsetoChannel _capsulecomponent "ECC_WorldStatic" "ECR_Block"))

(event Custom|CustomEvent
  ;[1 1 1] Remove actor
  (Actor|DestroyActor))

(event EventBeginPlay
  ;[1 1 1] Reset collision
  (Utilities|Time|SetTimerbyEvent (delegate Custom|SetCollision) 5.0)
  ;[1 1 1] Remove actor
  (Utilities|Time|SetTimerbyEvent (delegate Custom|CustomEvent) (Variables|Default|GetDespawnTime)))

(event EventTick
  (params (DeltaSeconds :type Float%20%28single-precision%29))
  ;[1 1 1] Make AI move towards the player
  (AI|AIMoveTo self "0, 0, 0" (Game|Player|GetPlayerPawn 0) 5.0 false))

(fn ConstructionScript)