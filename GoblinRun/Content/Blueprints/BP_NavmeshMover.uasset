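; BP_NavmeshMover is an actor that keeps the level's NavMeshBoundsVolume centered on the player pawn.
; BeginPlay caches the first player pawn and the volume, then binds the move event to a MoveNavmesh dispatcher.
; Tick calls that dispatcher every frame, setting the volume's root location to the pawn's.
; If either reference is missing, it prints an error and disables its tick.
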(event Custom|MoveNavmesh_Event
  ;[0 0 1] Move navmesh to player position
  (Transformation|SetWorldLocation (Variables|/Script/Engine.Actor|GetRootComponent (Variables|Default|GetNavmeshRef)) (Transformation|GetActorLocation (Variables|Default|GetPlayerRef)) false false))

(event EventBeginPlay
  ;[0 0 1] Set references and check if they are valid. Disable tick if they arent
  (bind _output_get (Variables|Default|SetPlayerRef (Game|Player|GetPlayerPawn 0)))
  (Utilities|IsValid _output_get
    (:Is%20Valid
      (bind _returnvalue (Actor|GetActorOfClass "/Script/NavigationSystem.NavMeshBoundsVolume"))
      (bind _output_get_2 (Variables|Default|SetNavmeshRef _returnvalue))
      (Utilities|IsValid _output_get_2
        (:Is%20Valid
          ;[0 0 1] Move navmesh to player position
          (EventDispatchers|BindEventtoMoveNavmesh (delegate Custom|MoveNavmesh_Event)))
        (:Is%20Not%20Valid
          (Development|PrintString "BP_NavmeshMover ERROR: No navmesh found in the level! Not executing code" true true "(R=1.000000,G=0.000000,B=0.000000,A=1.000000)" 2e+01)
          (Actor|Tick|SetActorTickEnabled false))))
    (:Is%20Not%20Valid
      (Development|PrintString "BP_NavmeshMover ERROR: No player found! Not executing code" true true "(R=1.000000,G=0.000000,B=0.000000,A=1.000000)" 2e+01)
      (Actor|Tick|SetActorTickEnabled false))))

(event EventTick
  (params (DeltaSeconds :type Float%20%28single-precision%29))
  ;[0 0 1] Execute event
  (Default|CallMoveNavmesh))

(fn ConstructionScript)