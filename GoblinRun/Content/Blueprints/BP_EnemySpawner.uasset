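; Enemy spawner that creates BP_Enemy actors on a looping timer, provided a player pawn exists at BeginPlay.
; Each spawn gets a random walk speed and side, with a random negative left or positive right value.
; Location comes from SetSpawnCoordinates, called separately per axis, though its randomly signed X/Y offsets from the player are computed but unused.
; Without a player, it prints an error and never starts the timer.
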(event Custom|EnemySpawn_Event
  (bind (_x _y _z) (Utilities|SetSpawnCoordinates))
  ;[1 1 1] Enemy spawn event
  (bind _returnvalue (Game|SpawnActorfromClass "/Game/Blueprints/BP_Enemy.BP_Enemy_C" (Math|Transform|MakeTransform (Math|Vector|MakeVector _x _y _z) "0, 0, 0" "1.000000,1.000000,1.000000") "Undefined" "MultiplyWithRoot" 0 0))
  ;[0 0 1] Set random variable values when spawning the enemy in
  (Utilities|IsValid _returnvalue
    (:Is%20Valid
      (Variables|/Script/Engine.CharacterMovementComponent|SetMaxWalkSpeed (Variables|/Script/Engine.Character|GetCharacterMovement _returnvalue) (Math|Random|RandomFloatinRange 1.2e+03 1.8e+03))
      (bind _output_get (Variables|/Game/Blueprints/BP_Enemy.BP_Enemy_C|SetLeftSide? _returnvalue (Math|Random|RandomBool)))
      (if _output_get
        (Variables|/Game/Blueprints/BP_Enemy.BP_Enemy_C|SetLeftValue _returnvalue (Math|Random|RandomFloatinRange -4e+02 -2e+02))
        (else
          (Variables|/Game/Blueprints/BP_Enemy.BP_Enemy_C|SetRightValue _returnvalue (Math|Random|RandomFloatinRange 2e+02 4e+02)))))))

(event EventBeginPlay
  ;[1 1 1] Get player ref
  (bind _output_get (Variables|Default|SetPlayerRef (Game|Player|GetPlayerPawn 0)))
  ;[1 1 1] Don't run event if the player isn't in the scene
  (Utilities|IsValid _output_get
    (:Is%20Valid
      (Utilities|Time|SetTimerbyEvent (delegate Custom|EnemySpawn_Event) (Variables|Default|GetEnemySpawnTime) true))
    (:Is%20Not%20Valid
      (Development|PrintString "BP_Enemyspawner ERROR: Player object not in scene! Not executing code in the enemy spawner." true true "(R=1.000000,G=0.000000,B=0.000000,A=1.000000)" 2e+01))))

(fn ConstructionScript)