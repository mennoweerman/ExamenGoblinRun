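; Enemy AI pawn that chases the player toward a point offset to one side and destroys itself after DespawnTime.
; At BeginPlay it picks that side by comparing world X of the player's left and right offset points.
; Tick reissues AIMoveTo toward the SetDestination point built from the player's right vector.
; Failed moves raise walk speed incrementally, while successful ones set it to a fixed value.
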(event Custom|DestroySelfEvent
  ;[1 1 1] Destroy self after a certain amount of time
  (Actor|DestroyActor))

(event EventBeginPlay
  (bind _movementoffset (Variables|Movement|GetMovementOffset))
  ;[1 1 1] Get player reference
  (Variables|References|SetPlayerRef (Game|Player|GetPlayerPawn 0))
  ;[1 1 1] Destroy self after a certain amount of time
  (Utilities|Time|SetTimerbyEvent (delegate Custom|DestroySelfEvent) (Variables|Despawning|GetDespawnTime))
  ;[1 1 1] Check if the left side of the player is closer to the spawn point of the AI. If so, move towards that side.
  (Variables|Movement|SetLeftSide? (< (.x (Utilities|CalculateSidewaysVectorfromPlayer (* _movementoffset -1.0))) (.x (Utilities|CalculateSidewaysVectorfromPlayer _movementoffset)))))

(event EventTick
  (params (DeltaSeconds :type Float%20%28single-precision%29))
  (bind _charactermovement (Variables|Character|GetCharacterMovement))
  ;[1 1 1] Move character towards the player
  (AI|AIMoveTo self (Utilities|SetDestination) 0 5.0 false
    (:OnSuccess
      ;[1 1 1] Make AI catch up and slow down when close by
      (Variables|/Script/Engine.CharacterMovementComponent|SetMaxWalkSpeed (Variables|Character|GetCharacterMovement) 1.2e+03))
    (:OnFail
      (Variables|/Script/Engine.CharacterMovementComponent|SetMaxWalkSpeed _charactermovement (+ (Variables|/Script/Engine.CharacterMovementComponent|GetMaxWalkSpeed _charactermovement) 1.0)))))

(fn ConstructionScript)