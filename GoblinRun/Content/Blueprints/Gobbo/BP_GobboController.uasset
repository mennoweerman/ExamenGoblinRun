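; BP_GobboController drives the player's Gobbo character with constant forward movement and left/right steering.
; BeginPlay adds the Enhanced Input mapping context and caches the player pawn and character.
; Tick forces movement input along the forward vector of MovementDirection, reached through the character's PlayerInputWidget, scaled by MovementSpeed.
; IA_Move only turns the pawn, feeding scaled X input into controller yaw while triggered or ongoing.
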(event Input|EnhancedActionEvents|EnhancedInputActionIA_Move
  (params (ActionValue :type Vector%202D%20Structure) (ElapsedSeconds :type Float%20%28double-precision%29) (TriggeredSeconds :type Float%20%28double-precision%29) (InputAction :type Input%20Action%20Object%20Reference :default "/Game/Blueprints/Gobbo/IA_Move.IA_Move"))
  ;[1 0 0] When Left or Right is pressed, adds one or minus one to the z input
  (:Triggered
    (Pawn|Input|AddControllerYawInput (Variables|References|GetPlayerPawnRef) (* (.x ActionValue) 1.3) :!label _label))
  (:Ongoing
    (goto _label)))

(event EventTick
  (params (DeltaSeconds :type Float%20%28single-precision%29))
  ;[1 1 1] Gets the players rotation, for the z it adds the rotation value and gets the forward vector to move the player in that direction using the movement speed
  (Pawn|Input|AddMovementInput (Variables|References|GetPlayerPawnRef) (Math|Vector|GetForwardVector (Transformation|GetWorldRotation (Variables|/Game/Blueprints/Widgets/W_PlayerInput.W_PlayerInput_C|GetMovementDirection (Variables|/Game/Blueprints/Gobbo/BP_GobboCharacter.BP_GobboCharacter_C|GetPlayerInputWidget (Variables|References|GetPlayerCharacterRef))))) (Variables|MovementSettings|GetMovementSpeed) true))

(event EventBeginPlay
  (bind _returnvalue (PlayerController|LocalPlayerSubsystems|GetEnhancedInputLocalPlayerSubsystem))
  ;[0.05098 0.05098 0.05098] Add Mapping Context
  (Utilities|IsValid _returnvalue
    (:Is%20Valid
      (Input|AddMappingContext _returnvalue "/Game/Blueprints/Gobbo/DA_GobboInputContextMapping.DA_GobboInputContextMapping" 0 "(bIgnoreAllPressedKeysUntilRelease=True,bForceImmediately=False,bNotifyUserSettings=False)")
      ;[1 1 1] Sets player pawn and player character references
      (Variables|References|SetPlayerPawnRef (Game|Player|GetPlayerPawn 0))
      (bind _asbp_gobbo_character (Utilities|Casting|CastToBP_GobboCharacter (Game|GetPlayerCharacter 0)))
      (Variables|References|SetPlayerCharacterRef _asbp_gobbo_character))))

(fn ConstructionScript)