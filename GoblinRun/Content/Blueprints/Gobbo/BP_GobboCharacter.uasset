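; BP_GobboCharacter is the rolling player character that takes damage from enemies and dies when health runs out.
; BeginPlay configures depth of field, creates input and data-manager widgets, starts game audio and loads or creates the save.
; Tick spins the model by velocity and toggles rolling sound.
; Enemy hits at low speed cost health, gated by a timer; death pauses the game, checks the highscore and switches the UI.
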(event OnComponentHit(CapsuleComponent)
  (params (HitComponent :type Primitive%20Component%20Object%20Reference) (OtherActor :type Actor%20Object%20Reference) (OtherComp :type Primitive%20Component%20Object%20Reference) (NormalImpulse :type Vector :default "0, 0, 0") (Hit :type Hit%20Result%20Structure%20%28by%20ref%29))
  ;[1 1 1] When the character is hit, check if the player gets hit by the enemy and is moving slower then 600cm/s. If true continue
  (if (and (== (Utilities|GetClass OtherActor) "/Game/Blueprints/Enemies/BP_Enemy.BP_Enemy_C") (<= (Math|Vector|VectorLength (Variables|/Script/Engine.MovementComponent|GetVelocity (Variables|Character|GetCharacterMovement))) (Variables|PlayerSettings|GetSpeedThreshold)))
    ;[1 1 1] When the hit timer is completed, remove 1 health point from the players health. Otherwise, start the hit timer
    (if (Variables|PlayerSettings|GetTimerCompleted?) :!label _label
      (bind _result (Math|Integer|DecrementInt (Variables|PlayerSettings|GetHealth))
        (:%20%20
          (if (<= _result 0)
            (CallFunction|PlayerDeath)
            (else
              (Variables|PlayerSettings|SetTimerCompleted? false)
              (goto _label_2 Reset)))))
      (else
        (Utilities|FlowControl|DoOnce false :!label _label_2
          (:Completed
            (CallFunction|HandleHitTimer)
            (goto _label)))))))

(event Custom|HandleHitTimer
  ;[1 1 1] Handles the hit timer
  (Utilities|Time|SetTimerbyEvent (delegate Custom|HitTimerOver) (Variables|PlayerSettings|GetTimeBeforeHit)))

(event Custom|HitTimerOver
  ;[1 1 1] Handles the hit timer
  (Variables|PlayerSettings|SetTimerCompleted? true))

(event EventBeginPlay
  ;[1 1 1] Handles the post process settings, then creates the player input and data manager widgets, sets their references and displays them on the screen.
  (Utilities|Struct|SetmembersinPostProcessSettings (Variables|/Script/Engine.PostProcessComponent|GetSettings (Variables|Default|GetPostProcess)) 0.035 65.0 (Variables|/Script/Engine.SpringArmComponent|GetTargetArmLength (Variables|Default|GetSpringArm)))
  (bind _returnvalue (UserInterface|CreateWidget "/Game/Blueprints/Widgets/W_PlayerInput.W_PlayerInput_C"))
  (bind _output_get (Variables|PlayerSettings|SetPlayerInputWidget _returnvalue))
  (UserInterface|Viewport|AddtoViewport _output_get 0)
  (bind _returnvalue_2 (UserInterface|CreateWidget "/Game/Blueprints/Widgets/Ingame/W_DataManager.W_DataManager_C"))
  (UserInterface|Viewport|AddtoViewport _returnvalue_2 0)
  ;[1 1 1] Hides the mouse cursor when the game begins
  (Variables|/Script/Engine.PlayerController|SetbShowMouseCursor (Game|GetPlayerController 0) false)
  ;[1 1 1] Gets the audio manager and plays the game sounds
  (bind _returnvalue_3 (Actor|GetActorOfClass "/Game/Blueprints/Gobbo/BP_AudioManager.BP_AudioManager_C"))
  (bind _output_get_2 (Variables|References|SetAudioManagerRef _returnvalue_3))
  (Default|PlayGameSounds _output_get_2)
  ;[1 1 1] Checks if the save file exists, if true load the game. Otherwise create a new save file
  (bind _returnvalue_4 (SaveGame|DoesSaveGameExist (Variables|PlayerSettings|GetSaveFileName)))
  (if _returnvalue_4
    (bind _returnvalue_5 (SaveGame|LoadGamefromSlot (Variables|PlayerSettings|GetSaveFileName)))
    (bind _assg_save_file (Utilities|Casting|CastToSG_SaveFile _returnvalue_5))
    (Variables|References|SetSaveFileRef _assg_save_file)
    (else
      (bind _returnvalue_6 (SaveGame|CreateSaveGameObject "/Game/Blueprints/Widgets/SG_SaveFile.SG_SaveFile_C"))
      (Variables|References|SetSaveFileRef _returnvalue_6))))

(event EventTick
  (params (DeltaSeconds :type Float%20%28single-precision%29))
  ;[1 1 1] Makes the player model roll
  (bind _result (Math|Float|NegateFloat (* (/ (Math|Vector|VectorLength (Variables|/Script/Engine.MovementComponent|GetVelocity (Variables|Character|GetCharacterMovement))) 2.0) (Variables|PlayerSettings|GetModelRotationSpeed) DeltaSeconds (Variables|PlayerSettings|GetRollingDirection)))
    (:%20%20
      (Transformation|AddLocalRotation (Variables|Default|GetGobbo) (Math|Rotator|MakeRotator 0.0 0.0 _result) false false)
      ;[1 1 1] Based on if the player is moving, play a rolling sound effect
      (if (>= (Math|Vector|VectorLength (Variables|/Script/Engine.MovementComponent|GetVelocity (Variables|Character|GetCharacterMovement))) 1e+02)
        (Utilities|FlowControl|DoOnce false :!label _label
          (:Completed
            (bind _returnvalue (AddComponent|AddAudioComponent false))
            (bind _output_get (Variables|Default|SetRollAudio _returnvalue))
            (Audio|Components|Audio|SetSound _output_get "/Game/Movies/Audio/RollingBarrelSound.RollingBarrelSound")
            (Audio|Components|Audio|Play _output_get 0.0)))
        (else
          (Utilities|IsValid (Variables|Default|GetRollAudio)
            (:Is%20Valid
              (Audio|Components|Audio|Stop (Variables|Default|GetRollAudio))
              (goto _label Reset))))))))

(fn ConstructionScript)

(fn PlayerDeath
  ;[1 1 1] Handles the player death
  (Game|SetGamePaused true)
  (Variables|/Script/Engine.PlayerController|SetbShowMouseCursor (Game|GetPlayerController 0) true)
  (Default|HandlePauseButtonSettings (Variables|References|GetDataManagerWidgetRef) 0.0 false)
  (Default|CheckforNewHighscore (Variables|References|GetDataManagerWidgetRef) (Variables|References|GetSaveFileRef))
  (Default|HandleScoreTexts (Variables|References|GetDataManagerWidgetRef))
  (Variables|/Script/UMG.WidgetSwitcher|SetActiveWidgetIndex (Variables|/Game/Blueprints/Widgets/Ingame/W_DataManager.W_DataManager_C|GetWidgetSwitcher (Variables|References|GetDataManagerWidgetRef)) 3)
  (Default|PlayDeathAudio (Variables|References|GetAudioManagerRef)))