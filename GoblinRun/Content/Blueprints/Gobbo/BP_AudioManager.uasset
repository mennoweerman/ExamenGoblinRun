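; BP_AudioManager switches the 2D music between the main menu and gameplay in a goblin runner game.
; PlayGameSounds fades out any valid menu audio over one second, then creates and plays the game sound.
; PlayDeathAudio does the reverse, fading out the game audio and starting the main menu track on death.
; Each newly created audio component is stored in a variable so the opposite event can fade it out.
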(event Custom|PlayDeathAudio
  ;[0 0 1] Event that fades out the game sounds and starts playing the main menu audio
  (Utilities|IsValid (Variables|Default|GetGameAudio)
    (:Is%20Valid
      (Audio|Components|Audio|FadeOut (Variables|Default|GetGameAudio) 1.0 0.3 "Linear" :!class /Script/Engine.AudioComponent))
    (:Is%20Not%20Valid
      _))
  (bind _returnvalue (Audio|CreateSound2D "/Game/Movies/Audio/MainMenuSoundGoblinRun.MainMenuSoundGoblinRun" 0.2 1.0 0.0 0))
  (bind _output_get (Variables|Default|SetMainMenuAudio _returnvalue))
  (Audio|Components|Audio|Play _output_get 0.0))

(event Custom|PlayGameSounds
  ;[0 0 1] Event that fades out the main menu sound and starts playing the game audio
  (Utilities|IsValid (Variables|Default|GetMainMenuAudio)
    (:Is%20Valid
      (Audio|Components|Audio|FadeOut (Variables|Default|GetMainMenuAudio) 1.0 0.3 "Linear" :!class /Script/Engine.AudioComponent))
    (:Is%20Not%20Valid
      _))
  (bind _returnvalue (Audio|CreateSound2D "/Game/Movies/Audio/GoblinGameSound.GoblinGameSound" 1.0 1.0 0.0 0))
  (bind _output_get (Variables|Default|SetGameAudio _returnvalue))
  (Audio|Components|Audio|Play _output_get 0.0))

(fn ConstructionScript)