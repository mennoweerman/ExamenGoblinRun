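; BP_Enemy is an AI enemy that moves toward a point offset to one side of the player.
; On BeginPlay it caches the player pawn and chooses left or right by comparing only the world X of both offset points, not their distance to the enemy.
; Every Tick it reissues AI MoveTo to the chosen side, recomputed from the player's current location and right vector scaled by MovementOffset.
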(event EventBeginPlay
  (bind _movementoffset (Variables|Movement|GetMovementOffset))
  ;[1 1 1] Get player reference
  (Variables|References|SetPlayerRef (Game|Player|GetPlayerPawn 0))
  ;[1 1 1] Check if the left side of the player is closer to the spawn point of the AI. If so, move towards that side.
  (Variables|Movement|SetLeftSide? (< (.x (Utilities|CalculateSidewaysVectorfromPlayer (* _movementoffset -1.0))) (.x (Utilities|CalculateSidewaysVectorfromPlayer _movementoffset)))))

(event EventTick
  (params (DeltaSeconds :type Float%20%28single-precision%29))
  ;[1 1 1] Move character towards the player
  (AI|AIMoveTo self (Utilities|SetDestination) 0 5.0 false))

(fn ConstructionScript)