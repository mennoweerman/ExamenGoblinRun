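; BP_EnemySpawner spawns waves of BP_Enemy that escalate with a wanted level, and disables itself if no player pawn exists.
; A one-shot BeginPlay timer starts the wave event, which re-triggers through delayed calls and doubles the spawn interval after its loop.
; GetWaveData advances the wanted-level enum until capped, reading enemy count and speed from EnemyMap.
; Each enemy spawns at SetSpawnCoordinates with that value as walk speed and acceleration.
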(event Custom|EnemySpawn_Event
  ;[1 1 1] Spawn enemies in wave according to the wanted system
  (bind (_amountofenemies _movementspeedandaccel) (CallFunction|GetWaveData))
  (for _index (range 0 _amountofenemies)
    (CallFunction|SpawnEnemyandSetVariables _movementspeedandaccel)
    (Utilities|FlowControl|Delay (Variables|Spawning|GetEnemySpawnTime))
    (CallFunction|EnemySpawnEvent))
  (Variables|Spawning|SetEnemySpawnTime (+ (Variables|Spawning|GetEnemySpawnTime) (Variables|Spawning|GetEnemySpawnTime))))

(event EventBeginPlay
  ;[1 1 1] Get player ref
  (bind _output_get (Variables|References|SetPlayerRef (Game|Player|GetPlayerPawn 0)))
  ;[1 1 1] Don't run event if the player isn't in the scene
  (Utilities|IsValid _output_get
    (:Is%20Valid
      ;[1 1 1] Spawn enemies in wave according to the wanted system
      (Utilities|Time|SetTimerbyEvent (delegate Custom|EnemySpawn_Event) (Variables|Spawning|GetEnemySpawnTime)))
    (:Is%20Not%20Valid
      (Development|PrintString "BP_Enemyspawner ERROR: Player object not in scene! Not executing code in the enemy spawner." true true "(R=1.000000,G=0.000000,B=0.000000,A=1.000000)" 2e+01)
      (Actor|Tick|SetActorTickEnabled false))))

(fn ConstructionScript)

(fn SpawnEnemyandSetVariables
  (params (MovementValue :type Float%20%28double-precision%29))
  (bind (_x _y _z) (Utilities|SetSpawnCoordinates))
  ;[0 0 1] Spawn enemy and set variables
  (bind _returnvalue (Game|SpawnActorfromClass "/Game/Blueprints/Enemies/BP_Enemy.BP_Enemy_C" (Math|Transform|MakeTransform (Math|Vector|MakeVector _x _y _z) "0, 0, 0" "1.000000,1.000000,1.000000") "Undefined" "MultiplyWithRoot" 0 0))
  (Utilities|IsValid _returnvalue
    (:Is%20Valid
      (bind _output_get (Variables|/Script/Engine.CharacterMovementComponent|SetMaxWalkSpeed (Variables|/Script/Engine.Character|GetCharacterMovement _returnvalue) MovementValue))
      (Variables|/Script/Engine.CharacterMovementComponent|SetMaxAcceleration (Variables|/Script/Engine.Character|GetCharacterMovement _returnvalue) _output_get)
      (return))))

(fn GetWaveData
  ;[0 0 1] Get wave datafrom the map
  (switch Utilities|FlowControl|Switch|SwitchonE_WantedLevel (Utilities|Enum|ByteToEnumE_WantedLevel (+ (Variables|Default|GetWantedLevelEnum) (Variables|Default|GetValueForEnum)))
    (:NewEnumerator0
      _)
    (:NewEnumerator1
      _)
    (:NewEnumerator2
      _)
    (:NewEnumerator3
      _)
    (:NewEnumerator4
      (Variables|Default|SetValueForEnum 0)))
  (bind _output_get (Variables|Default|SetWantedLevelEnum (Utilities|Enum|ByteToEnumE_WantedLevel (+ (Variables|Default|GetWantedLevelEnum) (Variables|Default|GetValueForEnum)))))
  (return (.AmountOfEnemies (Utilities|Struct|BreakS_Wanted (.Value (Utilities|Map|Find (Variables|Default|GetEnemyMap) _output_get)))) (.MovementSpeedAndAccel (Utilities|Struct|BreakS_Wanted (.Value (Utilities|Map|Find (Variables|Default|GetEnemyMap) _output_get))))))