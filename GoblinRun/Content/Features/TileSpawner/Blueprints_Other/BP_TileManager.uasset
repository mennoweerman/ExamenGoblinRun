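; Tile manager Blueprint that sorts spawnable tile classes into per-side adjacency lists for later tile spawning.
; On BeginPlay, three functions build the land, road and water maps.
; Each loops over every side and tile class, reads the class defaults for that side's connection flag, and adds matching tiles to that side's possible-adjacent array.
; The map lookups rely on value order matching the side index.
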(event EventBeginPlay
  ;[1 1 1] Assigns tiles to the correct lists to use for spawning later.
  (CallFunction|AssignLandTiles)
  (CallFunction|AssignRoadTiles)
  (CallFunction|AssignWaterTiles))

(event Collision|EventActorBeginOverlap
  (params (OtherActor :type Actor%20Object%20Reference)))

(event EventTick
  (params (DeltaSeconds :type Float%20%28single-precision%29)))

(fn ConstructionScript)

(fn AssignLandTiles
  ;[1 1 1] Loops through all tiles and gets their default Possible Tile Connections. Gets the values of the Land connection. If it is true, the Tiles Land map is updated to include that tile.
  (for (_ _array_index) (Variables|TileLists|GetTileSides)
    (for _array_element (Variables|TileLists|GetAllSpawnableTiles)
      (bind _values (Utilities|Map|Values (Utilities|GetClassDefaults _array_element)))
      (if (.land (Utilities|Array|Get(acopy) _values _array_index))
        (bind _values_2 (Utilities|Map|Values (Variables|TileLists|GetTilesLand)))
        (bind _output_get (LocalVariables|SetArray (.possibleadjacenttiles (Utilities|Array|Get(acopy) _values_2 _array_index))))
        (Utilities|Array|Add _output_get _array_element)
        (Utilities|Map|Add (Variables|TileLists|GetTilesLand) (Utilities|Select :Index _array_index :Option%200 (Utilities|Enum|LiteralenumE_TileSides "NewEnumerator0") :Option%201 (Utilities|Enum|LiteralenumE_TileSides "NewEnumerator1") :Option%202 (Utilities|Enum|LiteralenumE_TileSides "NewEnumerator2") :Option%203 (Utilities|Enum|LiteralenumE_TileSides "NewEnumerator3")) (Utilities|Struct|MakeS_PossibleAdjacentTiles (LocalVariables|GetArray))))))
  (return))

(fn AssignRoadTiles
  ;[1 1 1] Loops through all tiles and gets their default Possible Tile Connections. Gets the values of the Road connection. If it is true, the Tiles Road map is updated to include that tile.
  (for (_ _array_index) (Variables|TileLists|GetTileSides)
    (for _array_element (Variables|TileLists|GetAllSpawnableTiles)
      (bind _values (Utilities|Map|Values (.PossibleTileConnections (Utilities|GetClassDefaults _array_element))))
      (if (.road (Utilities|Array|Get(acopy) _values _array_index))
        (bind _values_2 (Utilities|Map|Values (Variables|TileLists|GetTilesRoad)))
        (bind _output_get (LocalVariables|SetArray (.possibleadjacenttiles (Utilities|Array|Get(acopy) _values_2 _array_index))))
        (Utilities|Array|Add _output_get _array_element)
        (Utilities|Map|Add (Variables|TileLists|GetTilesRoad) (Utilities|Select :Index _array_index :Option%200 (Utilities|Enum|LiteralenumE_TileSides "NewEnumerator0") :Option%201 (Utilities|Enum|LiteralenumE_TileSides "NewEnumerator1") :Option%202 (Utilities|Enum|LiteralenumE_TileSides "NewEnumerator2") :Option%203 (Utilities|Enum|LiteralenumE_TileSides "NewEnumerator3")) (Utilities|Struct|MakeS_PossibleAdjacentTiles (LocalVariables|GetArray))))))
  (return))

(fn AssignWaterTiles
  ;[1 1 1] Loops through all tiles and gets their default Possible Tile Connections. Gets the values of the Water connection. If it is true, the Tiles Water map is updated to include that tile.
  (for (_ _array_index) (Variables|TileLists|GetTileSides)
    (for _array_element (Variables|TileLists|GetAllSpawnableTiles)
      (bind _values (Utilities|Map|Values (Utilities|GetClassDefaults _array_element)))
      (if (.water (Utilities|Array|Get(acopy) _values _array_index))
        (bind _values_2 (Utilities|Map|Values (Variables|TileLists|GetTilesWater)))
        (bind _output_get (LocalVariables|SetArray (.possibleadjacenttiles (Utilities|Array|Get(acopy) _values_2 _array_index))))
        (Utilities|Array|Add _output_get _array_element)
        (Utilities|Map|Add (Variables|TileLists|GetTilesWater) (Utilities|Select :Index _array_index :Option%200 (Utilities|Enum|LiteralenumE_TileSides "NewEnumerator0") :Option%201 (Utilities|Enum|LiteralenumE_TileSides "NewEnumerator1") :Option%202 (Utilities|Enum|LiteralenumE_TileSides "NewEnumerator2") :Option%203 (Utilities|Enum|LiteralenumE_TileSides "NewEnumerator3")) (Utilities|Struct|MakeS_PossibleAdjacentTiles (LocalVariables|GetArray))))))
  (return))